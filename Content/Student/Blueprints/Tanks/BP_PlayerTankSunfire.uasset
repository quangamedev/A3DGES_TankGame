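; BP_PlayerTankSunfire is a player tank variant whose ability is a burst of fire damage around the tank.
; It overrides Ability to apply full, non-falloff radial damage at its Sphere component's location and show the FireField component.
; EndAbility hides FireField again.
; Damage is applied once per Ability call, and the event graph holds only disabled default nodes.
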(fn `Ability`
  (returns (Success :type Boolean))
  (`GameplayStatics.ApplyRadialDamage` :`BaseDamage` 30.0 :`Origin` (`SceneComponent.K2_GetComponentLocation` (`self.Sphere`)) :`DamageRadius` 250.0 :`DamageCauser` self :`InstigatedByController` null :`bDoFullDamage` true)
  (`SceneComponent.SetVisibility` (`self.FireField`) true false)
  (return false))

(fn `EndAbility`
  (returns (Success :type Boolean))
  (`SceneComponent.SetVisibility` (`self.FireField`) false false)
  (return false))

(fn `UserConstructionScript`
  (`parent.UserConstructionScript`))