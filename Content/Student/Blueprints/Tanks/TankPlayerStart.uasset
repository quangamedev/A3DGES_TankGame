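; TankPlayerStart is a player start actor for the tank game, tagged with a Team value of Red or Blue.
; Its construction script switches on Team and colours the text render and arrow components red or blue to match.
; The event graph holds only disabled stub events, so the Blueprint adds no runtime logic.
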(fn `UserConstructionScript`
  (bind _textrender (`self.TextRender`))
  (bind _arrow (`self.Arrow`))
  (switch `/Game/Student/Blueprints/Tanks/TeamsList` (`self.Team`)
    (:`NewEnumerator1`
      (`TextRenderComponent.SetTextRenderColor` _textrender (make `Color` 0 0 255))
      (set `ArrowComponent.ArrowColor` (make `Color` 0 0 255) _arrow))
    (:`NewEnumerator2`
      (`TextRenderComponent.SetTextRenderColor` _textrender (make `Color` 255))
      (set `ArrowComponent.ArrowColor` (make `Color` 255) _arrow))))