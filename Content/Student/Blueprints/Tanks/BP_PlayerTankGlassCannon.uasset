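; Glass cannon variant of the player tank, a child Blueprint that overrides weapon setup and the special ability.
; Weapon setup passes a fixed, boosted attack multiplier to the parent, ignoring the incoming value.
; The ability jumps the root a short distance along the tank's facing without sweeping for collision and switches to the ability move speed.
; Ending the ability restores base speed; the event graph adds no logic.
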(fn `Ability`
  (returns (Success :type Boolean))
  (`SceneComponent.K2_AddRelativeLocation` (`self.DefaultSceneRoot`) (* (`KismetMathLibrary.Conv_RotatorToVector` (`SceneComponent.K2_GetComponentRotation` (`self.Tank`))) 200.0) false false)
  (set `self.MoveSpeed` (`self.AbilityMoveSpeed`))
  (return false))

(fn `EndAbility`
  (returns (Success :type Boolean))
  (set `self.MoveSpeed` (`self.BaseMoveSpeed`))
  (return false))

(fn `SetupWeaponAttributes`
  (params (AttackMultiplier :type "Float (double-precision)"))
  (`parent.SetupWeaponAttributes` 1.6))

(fn `UserConstructionScript`
  (`parent.UserConstructionScript`))