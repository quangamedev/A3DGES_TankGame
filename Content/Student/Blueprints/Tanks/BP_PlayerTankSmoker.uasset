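; Player tank variant whose ability lays down smoke at the tank's current location.
; The Ability input spawns three big smoke emitters in a staggered burst, destroys them together after a few seconds, then re-arms a DoOnce gate after a short delay.
; It passes a fixed, above-one attack multiplier to the parent weapon setup.
; The Ability and EndAbility functions are empty, as the logic lives in the event graph.
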(event `InputAction|Ability`
  (params (Key :type "Key Structure"))
  (bind _returnvalue (`SceneComponent.K2_GetComponentLocation` (`self.Tank`)))
  (:`Pressed`
    (`/Engine/EditorBlueprintResources/StandardMacros.DoOnce` false :!label _label
      (:`Completed`
        (bind _returnvalue_2 (`GameplayStatics.SpawnEmitterAtLocation` "/Game/LowPoly_Universe/FX/P_Smoke_big.P_Smoke_big" _returnvalue))
        (`KismetSystemLibrary.Delay` 0.5)
        (bind _returnvalue_3 (`GameplayStatics.SpawnEmitterAtLocation` "/Game/LowPoly_Universe/FX/P_Smoke_big.P_Smoke_big" _returnvalue))
        (`KismetSystemLibrary.Delay` 0.5)
        (bind _returnvalue_4 (`GameplayStatics.SpawnEmitterAtLocation` "/Game/LowPoly_Universe/FX/P_Smoke_big.P_Smoke_big" _returnvalue))
        (`KismetSystemLibrary.Delay` 5.0)
        (`|ExecutionSequence`
          (:`then_0`
            (`ActorComponent.K2_DestroyComponent` _returnvalue_2)
            (`KismetSystemLibrary.Delay` 0.8)
            (goto _label :!via `Reset`))
          (:`then_1`
            (`ActorComponent.K2_DestroyComponent` _returnvalue_3))
          (:`then_2`
            (`ActorComponent.K2_DestroyComponent` _returnvalue_4)))))))

(fn `Ability`
  (returns (Success :type Boolean)))

(fn `EndAbility`
  (returns (Success :type Boolean)))

(fn `SetupWeaponAttributes`
  (params (AttackMultiplier :type "Float (double-precision)"))
  (`parent.SetupWeaponAttributes` 1.2))

(fn `UserConstructionScript`
  (`parent.UserConstructionScript`))