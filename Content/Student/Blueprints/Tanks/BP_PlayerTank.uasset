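; BP_PlayerTank is the player-controlled tank, with movement, health, death, a weapon inventory and placeholder ability functions, apparently for child tanks to override.
; Input drives body movement and rotation, and forwards turret turning and firing as messages to the TurretMountPoint child actor, whose class can be swapped.
; An Inventory handles pickup, cycling and dropping, with pickups raising the mounted weapon's attack multiplier.
; A DoOnce with delays times the ability and its cooldown.
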(event `self.ReceiveBeginPlay`
  ;[1 1 1] set the weapon attributes for child tanks
  (`self.SetupWeaponAttributes` 1.0))

(event `InputAxis|RotateRight`
  (params (AxisValue :type "Float (single-precision)"))
  (bind _tankrotation (`self.TankRotation`))
  (bind _tankrotatespeed (`self.TankRotateSpeed`))
  (bind _returnvalue (`KismetMathLibrary.MakeRotator` 0.0 0.0 (`self.TankRotation`)))
  ;[1 1 1] Tanks Movement and actions
  ;;[1 1 1] Handles the tanks duration
  (`/Engine/EditorBlueprintResources/StandardMacros.CompareFloat` AxisValue
    (:`>`
      (`SceneComponent.K2_SetWorldRotation` (`self.DefaultSceneRoot`) _returnvalue false false)
      (set `self.TankRotation` (+ _tankrotation _tankrotatespeed)))
    (:`<`
      (`SceneComponent.K2_SetWorldRotation` (`self.DefaultSceneRoot`) _returnvalue false false)
      (set `self.TankRotation` (- _tankrotation _tankrotatespeed)))))

(event `InputAxis|MoveForward`
  (params (AxisValue :type "Float (single-precision)"))
  ;[1 1 1] Tanks Movement and actions
  ;;[1 1 1] Handles the tanks movement
  (`self.AddMovementInput` (`self.GetActorForwardVector`) (* AxisValue (`self.MoveSpeed`))))

(event `InputAxis|RotateWeaponRight`
  (params (AxisValue :type "Float (single-precision)"))
  ;[1 1 1] Tanks Movement and actions
  ;;[1 1 1] Handles to turrets rotation
  (message `/Game/Student/Blueprints/Interfaces/I_Weapon.Turn` (`ChildActorComponent.ChildActor` (`self.TurretMountPoint`)) AxisValue (`self.TurretRotateSpeed`)))

(event `InputAction|Fire`
  (params (Key :type "Key Structure"))
  (bind _childactor (`ChildActorComponent.ChildActor` (`self.TurretMountPoint`)))
  ;[1 1 1] Tanks Movement and actions
  ;;[1 1 1] Handles the tanks firing
  (:`Pressed`
    (message `/Game/Student/Blueprints/Interfaces/I_Weapon.FireWeapon` _childactor))
  (:`Released`
    (message `/Game/Student/Blueprints/Interfaces/I_Weapon.ReleaseFire` _childactor)))

(event `InputAction|Ability`
  (params (Key :type "Key Structure"))
  ;[1 1 1] Tanks Movement and actions
  ;;[1 1 1] The tanks special ability
  (:`Pressed`
    (`/Engine/EditorBlueprintResources/StandardMacros.DoOnce` false :!label _label
      (:`Completed`
        (`self.Ability`)
        (`KismetSystemLibrary.Delay` 1.0)
        (`self.EndAbility`)
        (`KismetSystemLibrary.Delay` 3.0)
        (goto _label :!via `Reset`)))))

(event `Death`
  ;[1 1 1] Tanks death
  (`Controller.UnPossess` (`self.GetController`))
  (`self.K2_DestroyActor`))

(event `AddHealth`
  (params (Amount :type "Float (double-precision)"))
  ;[1 1 1] Adding health to the tank
  (set `self.Health` (`KismetMathLibrary.FClamp` (+ Amount (`self.Health`)) 0.0 (`self.MaxHealth`))))

(event `self.ReceiveAnyDamage`
  (params (Damage :type "Float (single-precision)") (DamageType :type "DamageType Object Reference") (InstigatedBy :type "Controller Object Reference") (DamageCauser :type "Actor Object Reference"))
  ;[1 1 1] Tank taking damage
  (bind _output_get (set `self.Health` (- (`self.Health`) Damage)))
  (`KismetSystemLibrary.PrintString` (`KismetStringLibrary.Conv_DoubleToString` _output_get))
  (if (<= _output_get 0.0)
    (`self.Death`)))

(event `/Game/Student/Blueprints/Interfaces/I_Tank.WeaponPickedUp`
  (params (Weapon :type "/Game/Student/Blueprints/Weapons/BaseWeapon Class Reference"))
  ;[1 1 1] Picking up and item and put it into the inventory
  (`/Game/Student/Blueprints/Components/Inventory.PickedUp` (`self.Inventory`) Weapon)
  (`self.SetupWeaponAttributes` 2.0))

(event `/Game/Student/Blueprints/Interfaces/I_Tank.ChangeToWeapon`
  (params (ChangeTo :type "/Game/Student/Blueprints/Weapons/BaseWeapon Class Reference"))
  ;[1 1 1] Changing the turret mount point's weapon
  (`ChildActorComponent.SetChildActorClass` (`self.TurretMountPoint`) ChangeTo))

(event `InputAction|CycleUp`
  (params (Key :type "Key Structure"))
  ;[1 1 1] cycle up and down the items in the inventory
  (:`Pressed`
    (`/Game/Student/Blueprints/Components/Inventory.CycleUp` (`self.Inventory`))))

(event `InputAction|CycleDown`
  (params (Key :type "Key Structure"))
  ;[1 1 1] cycle up and down the items in the inventory
  (:`Pressed`
    (`/Game/Student/Blueprints/Components/Inventory.CycleDown` (`self.Inventory`))))

(event `Key|Y`
  (params (Key :type "Key Structure"))
  ;[1 1 1] dropping items in the inventory
  (:`Pressed`
    (`/Game/Student/Blueprints/Components/Inventory.Drop` (`self.Inventory`))))

(fn `Ability`
  (returns (Success :type Boolean))
  (return true))

(fn `EndAbility`
  (returns (Success :type Boolean))
  (return true))

(fn `GetMaxWeapons`
  (returns (MaxWeapons :type Integer))
  (return (`self.MaxWeapons`)))

(fn `I_HealthPickUp`
  (params (Amount :type "Float (double-precision)"))
  (returns (Success :type Boolean))
  (`self.AddHealth` Amount)
  (return false))

(fn `SetupWeaponAttributes`
  (params (AttackMultiplier :type "Float (double-precision)" :default 1.0))
  (bind _asbase_weapon (cast `/Game/Student/Blueprints/Weapons/BaseWeapon` (`ChildActorComponent.ChildActor` (`self.TurretMountPoint`))))
  (set `/Game/Student/Blueprints/Weapons/BaseWeapon.AttackMultiplier` (* 1.0 AttackMultiplier) _asbase_weapon))

(fn `UserConstructionScript`)