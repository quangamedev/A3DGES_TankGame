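; Scout variant of the player tank, with a dash ability followed by a change in move speed.
; Ability sweeps the tank a short distance along its velocity, or a shorter one along its facing when stationary, with emitters at both ends.
; It then applies the ability move speed until EndAbility restores the base speed.
; Weapon setup passes a fixed neutral attack multiplier to the parent, ignoring its input.
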(fn `Ability`
  (returns (Success :type Boolean))
  (bind _returnvalue (`self.GetVelocity`))
  (bind _tank (`self.Tank`))
  (`GameplayStatics.SpawnEmitterAtLocation` "/Game/Particles/ArtilieryFirePAR.ArtilieryFirePAR" (`SceneComponent.K2_GetComponentLocation` _tank) (struct) (3.0 3.0 3.0))
  (if (`KismetMathLibrary.NotEqualExactly_VectorVector` _returnvalue)
    (`SceneComponent.K2_AddRelativeLocation` (`self.Tank`) (* (`KismetMathLibrary.Normal` _returnvalue) 350.0) true false)
    (else
      (`SceneComponent.K2_AddRelativeLocation` (`self.Tank`) (* (`KismetMathLibrary.Conv_RotatorToVector` (`SceneComponent.K2_GetComponentRotation` _tank)) 200.0) true false)))
  (`GameplayStatics.SpawnEmitterAtLocation` "/Game/Particles/ArtilieryFirePAR.ArtilieryFirePAR" (`SceneComponent.K2_GetComponentLocation` (`self.Tank`)) (struct) (1.5 1.5 1.5))
  (set `self.MoveSpeed` (`self.AbilityMoveSpeed`))
  (return false))

(fn `EndAbility`
  (returns (Success :type Boolean))
  (set `self.MoveSpeed` (`self.BaseMoveSpeed`))
  (return false))

(fn `SetupWeaponAttributes`
  (params (AttackMultiplier :type "Float (double-precision)"))
  (`parent.SetupWeaponAttributes` 1.0))

(fn `UserConstructionScript`
  (`parent.UserConstructionScript`))