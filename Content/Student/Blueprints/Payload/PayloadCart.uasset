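; PayloadCart is a payload objective cart that moves forward or backward along the spline of a referenced track while its radar disc spins each tick.
; A timeline, rate-scaled by Duration, drives location and rotation by distance along the spline through Move and Stop events.
; Overlap detection is unfinished: the looping check timer and sphere overlap events are empty, Move and Stop calls are unwired, and GetHealth returns zero.
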(event `self.ReceiveBeginPlay`
  (`TimelineComponent.SetPlayRate` (`self.CartMover`) (/ 1.0 (`self.Duration`)))
  (`KismetSystemLibrary.K2_SetTimerDelegate` (delegate `CheckForOverlapActors`) 0.5 true))

(event `CheckForOverlapActors`)

(event `self.Move`
  (params (IsMovingForward :type Boolean))
  (bind _spline (`/Game/Student/Blueprints/Payload/PayloadTrack.Spline` (`self.PayloadTrackRef`)))
  (bind _returnvalue (`KismetMathLibrary.Lerp` 0.0 (`SplineComponent.GetSplineLength` _spline) (`self.Alpha`)))
  (if IsMovingForward
    (bind (_direction _alpha) (`Timeline|CartMover` :!label _label)
      (:`Update`
        (set `self.Alpha` _alpha)
        (`self.K2_SetActorLocationAndRotation` (`SplineComponent.GetLocationAtDistanceAlongSpline` _spline _returnvalue "World") (`SplineComponent.GetRotationAtDistanceAlongSpline` _spline _returnvalue "World"))))
    (else
      (goto _label :!via `Reverse`))))

(event `self.Stop`
  (goto _label :!via `Stop`))

(event `self.ReceiveTick`
  (params (DeltaSeconds :type "Float (single-precision)"))
  (`SceneComponent.K2_AddLocalRotation` (`self.RadarDisc`) (`KismetMathLibrary.MakeRotator` 0.0 0.0 (* DeltaSeconds (`self.RadarRotationRate`))) false false))

(event `self.Sphere.OnComponentBeginOverlap`
  (params (OverlappedComponent :type "PrimitiveComponent Object Reference") (OtherActor :type "Actor Object Reference") (OtherComp :type "PrimitiveComponent Object Reference") (OtherBodyIndex :type Integer) (bFromSweep :type Boolean) (SweepResult :type "HitResult Structure (by ref)")))

(event `self.Sphere.OnComponentEndOverlap`
  (params (OverlappedComponent :type "PrimitiveComponent Object Reference") (OtherActor :type "Actor Object Reference") (OtherComp :type "PrimitiveComponent Object Reference") (OtherBodyIndex :type Integer)))

(fn `GetHealth`
  (returns (Health :type "Float (double-precision)"))
  (return 0.0))

(fn `UserConstructionScript`)