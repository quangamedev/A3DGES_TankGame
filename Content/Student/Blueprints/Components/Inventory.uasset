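; Inventory component that stores an actor's collected weapons and handles equipping, cycling, dropping and clearing them.
; Pickups add unique entries and equip them immediately, but are ignored once the count reaches the maximum queried from the owner at BeginPlay.
; Cycling wraps around the array, and dropping equips the previous index if valid.
; Weapon changes reach the owner through message calls, keeping the component decoupled from its class.
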(event `PickedUp`
  (params (ItemPickedUp :type "/Game/Student/Blueprints/Weapons/BaseWeapon Class Reference"))
  ;[1 1 1] Picking up weapons
  (`self.WeaponCheck`
    (:`EmptyInventory`
      _)
    (:`HasWeapons`
      _))
  (bind _returnvalue (`KismetArrayLibrary.Array_AddUnique` (`self.Inventory`) ItemPickedUp)) ; add unique so we dont have duplicate weapons
  (if (!= _returnvalue -1)
    (`self.Equip` _returnvalue)))

(event `Equip`
  (params (ItemToEquipIndex :type Integer))
  ;[1 1 1] Equipping weapons
  (message `/Game/Student/Blueprints/Interfaces/I_Tank.ChangeToWeapon` (`self.GetOwner`) (`|GetArrayItem` (`self.Inventory`) ItemToEquipIndex))
  (set `self.EquippedWeapon` ItemToEquipIndex))

(event `CycleUp`
  ;[1 1 1] Cycyle up through weapons in inventory
  (bind _result (`/Engine/EditorBlueprintResources/StandardMacros.IncrementInt` (`self.EquippedWeapon`)) ; increase index
    (:`  `
      (if (`KismetArrayLibrary.Array_IsValidIndex` (`self.Inventory`) _result)
        (`self.Equip` _result)
        (else
          (`self.Equip` 0)
          (set `self.EquippedWeapon` 0))))))

(event `CycleDown`
  (bind _inventory (`self.Inventory`))
  (bind _returnvalue (`KismetArrayLibrary.Array_LastIndex` _inventory))
  ;[1 1 1] Cycle down through weapons in inventory
  (bind _result (`/Engine/EditorBlueprintResources/StandardMacros.DecrementInt` (`self.EquippedWeapon`)) ; decrease index
    (:`  `
      (if (`KismetArrayLibrary.Array_IsValidIndex` _inventory _result)
        (`self.Equip` _result)
        (else
          (`self.Equip` _returnvalue)
          (set `self.EquippedWeapon` _returnvalue))))))

(event `Drop`
  (bind _equippedweapon (`self.EquippedWeapon`))
  (bind _inventory (`self.Inventory`))
  ;[1 1 1] Drop the current weapon
  (if (`KismetArrayLibrary.Array_IsValidIndex` (`self.Inventory`) _equippedweapon)
    (`KismetArrayLibrary.Array_Remove` _inventory _equippedweapon)
    (bind _result (`/Engine/EditorBlueprintResources/StandardMacros.DecrementInt` _equippedweapon)
      (:`  `
        (if (`KismetArrayLibrary.Array_IsValidIndex` _inventory _result)
          (`self.Equip` _result))))))

(event `ClearAllItems`
  ;[1 1 1] Clear all items in the inventory
  (`KismetArrayLibrary.Array_Clear` (`self.Inventory`))
  (message `/Game/Student/Blueprints/Interfaces/I_Tank.ChangeToWeapon` (`self.GetOwner`) (`self.NoWeapon`)))

(event `self.ReceiveBeginPlay`
  (bind _maxweapons (message `/Game/Student/Blueprints/Interfaces/I_Tank.GetMaxWeapons` (`self.GetOwner`)))
  (set `self.MaxWeapons` _maxweapons))