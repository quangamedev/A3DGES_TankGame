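; Player controller for team deathmatch that holds a player's team, ready state, score and current tank class.
; On pawn death it waits briefly, requests a respawn from the game mode and credits the instigator unless it is self or a teammate.
; SpawnAndPossess spawns the given tank at a spawn spot, or at the current pawn's transform, and possesses it.
; It also toggles readiness on Start, reveals its respawn button and relays last-life buff messages.
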(event `/Game/Student/Blueprints/Interfaces/I_PlayerController.PawnDied`
  (params (Instigator :type "Controller Object Reference"))
  (`KismetSystemLibrary.Delay` 0.1) ; Delayed because destroyed actor is on the same tick as destroying the actor
  (bind _asteam_death_match_game_mode (cast `/Game/Student/Blueprints/GameModes/TeamDeathMatchGameMode` (`GameplayStatics.GetGameMode`))
    (:`then`
      (`/Game/Student/Blueprints/GameModes/TeamDeathMatchGameMode.RequestRespawn` _asteam_death_match_game_mode self)
      (bind _team (message `/Game/Student/Blueprints/Interfaces/I_PlayerController.GetTeam` Instigator))
      (bind _team_2 (`/Game/Student/Blueprints/Interfaces/I_PlayerController.GetTeam`))
      (if (and (`|EnumInequality` _team _team_2) (!= self Instigator))
        (`/Game/Student/Blueprints/GameModes/TeamDeathMatchGameMode.AddScoreTo` _asteam_death_match_game_mode Instigator)))
    (:`CastFailed`
      (`KismetSystemLibrary.PrintString` "Incorrect game mode to cast to"))))

(event `/Game/Student/Blueprints/Interfaces/I_PlayerController.LastLifeBuff`
  (while (not (`KismetSystemLibrary.IsValid` (`self.K2_GetPawn`)))
    _)
  (`KismetSystemLibrary.Delay` 0.2)
  (message `/Game/Student/Blueprints/Interfaces/I_Tank.LastLifeBuff` (`self.K2_GetPawn`)))

(event `InputAction|Start`
  (params (Key :type "Key Structure"))
  (:`Pressed`
    (bind _output_get (set `self.Ready` (not (`self.Ready`))))
    (`KismetSystemLibrary.PrintString` (`KismetStringLibrary.Conv_BoolToString` _output_get))))

(event `/Game/Student/Blueprints/Interfaces/I_PlayerController.EnableRespawnButton`
  (bind _foundwidgets (`WidgetBlueprintLibrary.GetAllWidgetsOfClass` "/Game/Student/Blueprints/Widgets/TeamDeathMatchUI.TeamDeathMatchUI_C"))
  (for _array_element _foundwidgets
    (if (== (`Widget.GetOwningPlayer` _array_element) self)
      (`Widget.SetVisibility` (`/Game/Student/Blueprints/Widgets/TeamDeathMatchUI.Respawn` _array_element) "Visible")
      (break))))

(event `/Game/Student/Blueprints/Interfaces/I_PlayerController.SetTeam`
  (params (Team :type "/Game/Student/Blueprints/Tanks/TeamsList Enum" :default "NewEnumerator0"))
  (set `self.Team` Team))

(event `/Game/Student/Blueprints/Interfaces/I_PlayerController.SetReadiness`
  (params (Readiness :type Boolean))
  (set `self.Ready` Readiness))

(fn `GetCurrentTank`
  (returns (CurrentTank :type "/Game/Student/Blueprints/Tanks/BP_BaseTank Class Reference"))
  (return (`self.CurrentTank`)))

(fn `GetLives`
  (returns (Lives :type Integer))
  (return 0))

(fn `GetScore`
  (returns (Score :type Integer))
  (return (`self.Score`)))

(fn `GetTeam`
  (returns (Team :type "/Game/Student/Blueprints/Tanks/TeamsList Enum"))
  (return (`self.Team`)))

(fn `IsReady`
  (returns (Ready :type Boolean))
  (return (`self.Ready`)))

(fn `SpawnAndPossess`
  (params (Tank :type "/Game/Student/Blueprints/Tanks/BP_BaseTank Class Reference") (`Spawn Spot` :type "Actor Object Reference"))
  (returns (SpawnedTank :type "/Game/Student/Blueprints/Tanks/BP_BaseTank Object Reference"))
  (locals (SpawnSpot :type "Actor Object Reference") (SpawnTransform :type "Transform Structure"))
  (bind _returnvalue (`self.K2_GetPawn` self))
  (bind _output_get (set `local.SpawnSpot` `Spawn Spot`))
  (`/Engine/EditorBlueprintResources/StandardMacros.IsValid` _output_get
    (:`Is Valid`
      (set `local.SpawnTransform` (`self.GetTransform` (`local.SpawnSpot`))))
    (:`Is Not Valid`
      (set `local.SpawnTransform` (`KismetMathLibrary.MakeTransform` (`self.K2_GetActorLocation` _returnvalue) (`self.K2_GetActorRotation` _returnvalue)))))
  (bind _output_get_2 (set `self.CurrentTank` Tank))
  (bind _returnvalue_2 (`|SpawnActorFromClass` _output_get_2 (`local.SpawnTransform`) "Undefined" "OverrideRootScale" self null))
  (`self.Possess` self _returnvalue_2)
  (return _returnvalue_2))

(fn `UserConstructionScript`)