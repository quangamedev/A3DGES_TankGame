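; Base laser weapon actor that fires two hitscan beams, from Arrow and RightArrow, repeatedly while fire is held.
; FireWeapon loops through a Gate and Firerate delay until ReleaseFire closes it, with a delayed DoOnce reset limiting re-presses.
; ShootRay spawns beam and hit particles, line-traces with debug drawing, and applies multiplied damage credited to the parent actor's instigator.
; Same-team hits deal damage only if the target reports positive health, assumed to be a cart.
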(event `/Game/Student/Blueprints/Interfaces/I_Weapon.FireWeapon`
  (bind _returnvalue (* (`self.Damage`) (`self.AttackMultiplier`)))
  (`/Engine/EditorBlueprintResources/StandardMacros.DoOnce` false :!label _label
    (:`Completed`
      (`|ExecutionSequence`
        (:`then_0`
          (goto _label_2 :!via `Open`))
        (:`then_1`
          (`/Engine/EditorBlueprintResources/StandardMacros.Gate` true :!label _label_2
            (:`Exit`
              (`self.ShootRay` (`self.Arrow`) _returnvalue)
              (`self.ShootRay` (`self.RightArrow`) _returnvalue)
              (`KismetSystemLibrary.Delay` (`self.Firerate`))
              (goto _label_2))))))))

(event `/Game/Student/Blueprints/Interfaces/I_Weapon.ReleaseFire`
  (`|ExecutionSequence`
    (:`then_0`
      (goto _label_2 :!via `Close`))
    (:`then_1`
      (`KismetSystemLibrary.Delay` (`self.Firerate`))
      (goto _label :!via `Reset`))))

(fn `ShootRay`
  (params (SpawnPosition :type "SceneComponent Object Reference") (Damage :type "Float (double-precision)"))
  (bind _returnvalue (`SceneComponent.K2_GetComponentLocation` SpawnPosition))
  (bind _returnvalue_2 (`self.GetInstigatorController` (`self.GetParentActor`)))
  (`GameplayStatics.SpawnEmitterAtLocation` "/Game/Particles/LaserBeamPAR.LaserBeamPAR" (`SceneComponent.K2_GetComponentLocation` SpawnPosition) (`SceneComponent.K2_GetComponentRotation` SpawnPosition))
  (bind (_outhit _returnvalue_3) (`KismetSystemLibrary.LineTraceSingle` :`Start` _returnvalue :`End` (+ _returnvalue (* (`SceneComponent.GetForwardVector` SpawnPosition) (`self.TraceDistance`))) :`TraceChannel` "TraceTypeQuery1" :`DrawDebugType` "ForDuration" :`DrawTime` 0.5))
  (if _returnvalue_3
    (bind (_bblockinghit _binitialoverlap _time _distance _location _impactpoint _normal _impactnormal _physmat _hitactor) (`GameplayStatics.BreakHitResult` _outhit))
    (`GameplayStatics.SpawnEmitterAtLocation` "/Game/Particles/LaserHitPAR.LaserHitPAR" _location)
    (bind _team (message `/Game/Student/Blueprints/Interfaces/I_PlayerController.GetTeam` (`self.GetOwner` _hitactor)))
    (bind _team_2 (message `/Game/Student/Blueprints/Interfaces/I_PlayerController.GetTeam` _returnvalue_2))
    (if (`|EnumInequality` _team _team_2)
      (`GameplayStatics.ApplyDamage` _hitactor Damage _returnvalue_2 self :!label _label)
      (else
        ;[1 1 1] if health > 0, object must be cart
        (bind _health (message `/Game/Student/Blueprints/Interfaces/I_PayloadCart.GetHealth` _hitactor))
        (if (> _health 0.0)
          (goto _label))))))

(fn `UserConstructionScript`
  (`parent.UserConstructionScript`))