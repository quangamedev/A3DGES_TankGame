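; BaseMortar is a weapon Blueprint that launches BaseMortarShell projectiles.
; FireWeapon and ReleaseFire drive a singleDelay node that paces shots by Firerate.
; On completion it spawns a shell at the Arrow transform, passes on AttackMultiplier and applies a Force-scaled impulse to the shell's Sphere along the Arrow's forward vector.
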(event `/Game/Student/Blueprints/Interfaces/I_Weapon.FireWeapon`
  (`/Game/Student/Blueprints/MacroLibraries/WeaponMacros.SingleDelay` (`self.Firerate`) :!label _label
    (:`Completed`
      (bind _returnvalue (`|SpawnActorFromClass` "/Game/Student/Blueprints/Weapons/Projectiles/BaseMortarShell.BaseMortarShell_C" (`SceneComponent.K2_GetComponentToWorld` (`self.Arrow`)) "Undefined" "OverrideRootScale" null null))
      (set `/Game/Student/Blueprints/Weapons/Projectiles/BaseMortarShell.AttackMultiplier` (`self.AttackMultiplier`) _returnvalue)
      (`PrimitiveComponent.AddImpulse` (`/Game/Student/Blueprints/Weapons/Projectiles/BaseMortarShell.Sphere` _returnvalue) (* (`KismetMathLibrary.Conv_RotatorToVector` (`SceneComponent.K2_GetComponentRotation` (`self.Arrow`))) (`self.Force`)) "None" false))))

(event `/Game/Student/Blueprints/Interfaces/I_Weapon.ReleaseFire`
  (goto _label :!via `Release`))

(fn `UserConstructionScript`
  (`parent.UserConstructionScript`))