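; Base explosive weapon Blueprint that fires missile projectiles, built on a parent weapon class.
; FireWeapon drives an automaticDelay by fire rate, and ReleaseFire releases it.
; When the delay completes, it spawns a missile at the Arrow component's world transform and passes it with the attack multiplier to SetProjectileDamage, which defers to the parent implementation.
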(event `self.ReceiveBeginPlay`
  (`parent.ReceiveBeginPlay`))

(event `/Game/Student/Blueprints/Interfaces/I_Weapon.FireWeapon`
  (`/Game/Student/Blueprints/MacroLibraries/WeaponMacros.AutomaticDelay` (`self.Firerate`) :!label _label
    (:`Completed`
      (bind _returnvalue (`|SpawnActorFromClass` "/Game/Student/Blueprints/Weapons/Projectiles/BaseMissile.BaseMissile_C" (`SceneComponent.K2_GetComponentToWorld` (`self.Arrow`)) "Undefined" "OverrideRootScale" null null))
      (`self.SetProjectileDamage` _returnvalue (`self.AttackMultiplier`)))))

(event `/Game/Student/Blueprints/Interfaces/I_Weapon.ReleaseFire`
  (goto _label :!via `Release`))

(fn `SetProjectileDamage`
  (params (Projectile :type "/Game/Student/Blueprints/Weapons/Projectiles/BaseProjectile Object Reference") (Multiplier :type "Float (double-precision)"))
  (`parent.SetProjectileDamage` Projectile Multiplier))

(fn `UserConstructionScript`
  (`parent.UserConstructionScript`))