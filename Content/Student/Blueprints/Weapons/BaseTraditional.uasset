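; BaseTraditional is a weapon Blueprint that fires projectiles from its Arrow component.
; FireWeapon passes through a singleDelay timed by Firerate, then spawns a BaseProjectile at the arrow's transform, and ReleaseFire releases that delay.
; Each valid projectile gets damage scaled by AttackMultiplier and a team taken from the parent actor's instigator controller.
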(event `/Game/Student/Blueprints/Interfaces/I_Weapon.FireWeapon`
  (`/Game/Student/Blueprints/MacroLibraries/WeaponMacros.SingleDelay` (`self.Firerate`) :!label _label
    (:`Completed`
      (bind _returnvalue (`|SpawnActorFromClass` "/Game/Student/Blueprints/Weapons/Projectiles/BaseProjectile.BaseProjectile_C" (`SceneComponent.K2_GetComponentToWorld` (`self.Arrow`)) "Undefined" "OverrideRootScale" null null))
      (bind _output_get (set `self.LatestProjectile` _returnvalue))
      (`/Engine/EditorBlueprintResources/StandardMacros.IsValid` _output_get
        (:`Is Valid`
          (`self.SetProjectileDamage` (`self.LatestProjectile`) (`self.AttackMultiplier`))
          (bind _team (message `/Game/Student/Blueprints/Interfaces/I_PlayerController.GetTeam` (`self.GetInstigatorController` (`self.GetParentActor`))))
          (`/Game/Student/Blueprints/Interfaces/I_Projectile.SetTeam` (`self.LatestProjectile`) _team))))))

(event `/Game/Student/Blueprints/Interfaces/I_Weapon.ReleaseFire`
  (goto _label :!via `Release`))

(fn `UserConstructionScript`
  (`parent.UserConstructionScript`))