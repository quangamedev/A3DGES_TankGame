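; Player turret Blueprint, filed under Old weapons, that rotates its Cube component from player input.
; Axis events share logic that builds a direction from the axis value and, past a deadzone, interpolates world rotation toward it.
; Tick and the left/right action events share key checks that increment or decrement TurnSpeed and apply it directly as absolute yaw, so this turning is frame-rate dependent.
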(event `InputAxis|RotateTurretX`
  (params (AxisValue :type "Float (single-precision)"))
  (bind _returnvalue (`KismetMathLibrary.MakeVector` AxisValue (* (stale `InputAxis|RotateTurretY` AxisValue) -1.0)))
  (if (> (`KismetMathLibrary.VSize` _returnvalue) 0.25) :!label _label
    (set `self.DestRot` (`KismetMathLibrary.Conv_VectorToRotator` _returnvalue))
    (`SceneComponent.K2_SetWorldRotation` (`self.Cube`) (`KismetMathLibrary.RInterpTo` (`SceneComponent.K2_GetComponentRotation` (`self.Cube`)) (`self.DestRot`) (`GameplayStatics.GetWorldDeltaSeconds`) 2.0) false false)))

(event `InputAxis|RotateTurretY`
  (params (AxisValue :type "Float (single-precision)"))
  (goto _label))

(event `self.ReceiveTick`
  (params (DeltaSeconds :type "Float (single-precision)"))
  (bind _returnvalue (`GameplayStatics.GetPlayerController` 0))
  (bind _turnspeed (`self.TurnSpeed`))
  (bind _cube (`self.Cube`))
  (if (`PlayerController.IsInputKeyDown` _returnvalue (stale `InputAction|RotateTurretRight` Key)) :!label _label_2
    (bind _result (`/Engine/EditorBlueprintResources/StandardMacros.IncrementFloat` _turnspeed)
      (:`  `
        (`SceneComponent.K2_SetWorldRotation` _cube (`KismetMathLibrary.MakeRotator` 0.0 0.0 _result) false false)))
    (elif (`PlayerController.IsInputKeyDown` _returnvalue (stale `InputAction|RotateTurretLeft` Key))
      (bind _result_2 (`/Engine/EditorBlueprintResources/StandardMacros.DecrementFloat` _turnspeed)
        (:`  `
          (`SceneComponent.K2_SetWorldRotation` _cube (`KismetMathLibrary.MakeRotator` 0.0 0.0 _result_2) false false))))))

(event `InputAction|RotateTurretRight`
  (params (Key :type "Key Structure"))
  (:`Pressed`
    (goto _label_2)))

(event `InputAction|RotateTurretLeft`
  (params (Key :type "Key Structure"))
  (:`Pressed`
    (goto _label_2)))

(fn `UserConstructionScript`)