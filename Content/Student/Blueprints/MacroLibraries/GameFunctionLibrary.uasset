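; Blueprint function library of shared helpers for the tank game's player setup and UI lookup.
; GetRandomTankClass picks one of five player tank classes at random.
; EquipAllWeapons and EquipRandomWeapon grant weapon classes through the tank's weapon pickup calls, with a flag that can exclude the traditional weapon from the random roll.
; GetControllersWidget searches top-level widgets of a class for the one owned by a given player controller.
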(fn `EquipAllWeapons`
  (params (Tank :type "/Game/Student/Blueprints/Tanks/BP_BaseTank Object Reference"))
  (message `/Game/Student/Blueprints/Interfaces/I_Tank.WeaponPickedUp` Tank "/Game/Student/Blueprints/Weapons/BaseExplosive.BaseExplosive_C")
  (message `/Game/Student/Blueprints/Interfaces/I_Tank.WeaponPickedUp` Tank "/Game/Student/Blueprints/Weapons/BaseLaser.BaseLaser_C")
  (message `/Game/Student/Blueprints/Interfaces/I_Tank.WeaponPickedUp` Tank "/Game/Student/Blueprints/Weapons/BaseMortar.BaseMortar_C")
  (message `/Game/Student/Blueprints/Interfaces/I_Tank.WeaponPickedUp` Tank "/Game/Student/Blueprints/Weapons/BaseTraditional.BaseTraditional_C")
  (message `/Game/Student/Blueprints/Interfaces/I_Tank.WeaponPickedUp` Tank "/Game/Student/Blueprints/Weapons/BaseWeapon.BaseWeapon_C"))

(fn `EquipRandomWeapon`
  (params (Tank :type "/Game/Student/Blueprints/Tanks/BP_BaseTank Object Reference") (IncludeTraditional :type Boolean :default true))
  (locals (WeaponClass :type "/Game/Student/Blueprints/Weapons/BaseWeapon Class Reference") (RandomRangeMax :type Integer :default 4))
  (`|ExecutionSequence`
    (:`then_0`
      (if (not IncludeTraditional)
        (set `local.RandomRangeMax` 3))
      (switch `int` (`KismetMathLibrary.RandomIntegerInRange` 0 (`local.RandomRangeMax`))
        (:`0`
          (set `local.WeaponClass` "/Game/Student/Blueprints/Weapons/BaseExplosive.BaseExplosive_C"))
        (:`1`
          (set `local.WeaponClass` "/Game/Student/Blueprints/Weapons/BaseLaser.BaseLaser_C"))
        (:`2`
          (set `local.WeaponClass` "/Game/Student/Blueprints/Weapons/BaseMortar.BaseMortar_C"))
        (:`3`
          (set `local.WeaponClass` "/Game/Student/Blueprints/Weapons/BaseWeapon.BaseWeapon_C"))
        (:`4`
          (set `local.WeaponClass` "/Game/Student/Blueprints/Weapons/BaseTraditional.BaseTraditional_C"))))
    (:`then_1`
      (`/Game/Student/Blueprints/Interfaces/I_Tank.WeaponPickedUp` Tank (`local.WeaponClass`)))))

(fn `GetControllersWidget`
  (params (WidgetClass :type "UserWidget Class Reference") (PlayerController :type "PlayerController Object Reference"))
  (returns (Widget :type "UserWidget Object Reference"))
  (bind _foundwidgets (`WidgetBlueprintLibrary.GetAllWidgetsOfClass` null WidgetClass))
  (for _array_element _foundwidgets
    (if (== (`Widget.GetOwningPlayer` _array_element) PlayerController)
      (return _array_element)))
  (return null))

(fn `GetRandomTankClass`
  (returns (TankClassRef :type "/Game/Student/Blueprints/Tanks/BP_BaseTank Class Reference"))
  (locals (TankClass :type "/Game/Student/Blueprints/Tanks/BP_BaseTank Class Reference"))
  (`|ExecutionSequence`
    (:`then_0`
      (switch `int` (`KismetMathLibrary.RandomIntegerInRange` 0 4)
        (:`0`
          (set `local.TankClass` "/Game/Student/Blueprints/Tanks/BP_PlayerTankGlassCannon.BP_PlayerTankGlassCannon_C"))
        (:`1`
          (set `local.TankClass` "/Game/Student/Blueprints/Tanks/BP_PlayerTankScout.BP_PlayerTankScout_C"))
        (:`2`
          (set `local.TankClass` "/Game/Student/Blueprints/Tanks/BP_PlayerTankSiege.BP_PlayerTankSiege_C"))
        (:`3`
          (set `local.TankClass` "/Game/Student/Blueprints/Tanks/BP_PlayerTankSmoker.BP_PlayerTankSmoker_C"))
        (:`4`
          (set `local.TankClass` "/Game/Student/Blueprints/Tanks/BP_PlayerTankSunfire.BP_PlayerTankSunfire_C"))))
    (:`then_1`
      (return (`local.TankClass`)))))