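; GameFunctionMacros is a macro library of shared gameplay helpers for tank selection and loadout.
; GetRandomTankClass rolls a random integer to pick one of five player tank Blueprint classes: Glass Cannon, Scout, Siege, Smoker or Sunfire.
; EquipAllWeapons sends the WeaponPickedUp interface message to a given tank once for each base weapon type, including the generic BaseWeapon.
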(fn `EquipAllWeapons`
  (params (Tank :type "/Game/Student/Blueprints/Tanks/BP_BaseTank Object Reference"))
  (message `/Game/Student/Blueprints/Interfaces/I_Tank.WeaponPickedUp` Tank "/Game/Student/Blueprints/Weapons/BaseExplosive.BaseExplosive_C")
  (message `/Game/Student/Blueprints/Interfaces/I_Tank.WeaponPickedUp` Tank "/Game/Student/Blueprints/Weapons/BaseLaser.BaseLaser_C")
  (message `/Game/Student/Blueprints/Interfaces/I_Tank.WeaponPickedUp` Tank "/Game/Student/Blueprints/Weapons/BaseMortar.BaseMortar_C")
  (message `/Game/Student/Blueprints/Interfaces/I_Tank.WeaponPickedUp` Tank "/Game/Student/Blueprints/Weapons/BaseTraditional.BaseTraditional_C")
  (message `/Game/Student/Blueprints/Interfaces/I_Tank.WeaponPickedUp` Tank "/Game/Student/Blueprints/Weapons/BaseWeapon.BaseWeapon_C"))

(fn `GetRandomTankClass`
  (returns (TankClassRef :type "/Game/Student/Blueprints/Tanks/BP_BaseTank Class Reference"))
  (locals (TankClass :type "/Game/Student/Blueprints/Tanks/BP_BaseTank Class Reference"))
  (switch `int` (`KismetMathLibrary.RandomIntegerInRange` 0 4)
    (:`0`
      (set `local.TankClass` "/Game/Student/Blueprints/Tanks/BP_PlayerTankGlassCannon.BP_PlayerTankGlassCannon_C"))
    (:`1`
      (set `local.TankClass` "/Game/Student/Blueprints/Tanks/BP_PlayerTankScout.BP_PlayerTankScout_C"))
    (:`2`
      (set `local.TankClass` "/Game/Student/Blueprints/Tanks/BP_PlayerTankSiege.BP_PlayerTankSiege_C"))
    (:`3`
      (set `local.TankClass` "/Game/Student/Blueprints/Tanks/BP_PlayerTankSmoker.BP_PlayerTankSmoker_C"))
    (:`4`
      (set `local.TankClass` "/Game/Student/Blueprints/Tanks/BP_PlayerTankSunfire.BP_PlayerTankSunfire_C")))
  (return (`local.TankClass`)))