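; Game mode for local multiplayer tank deathmatch that creates players and their DeathMatchUI screens.
; The match starts when all controllers are ready and ends when a retriggerable-delay countdown expires.
; Spawns use random tanks at team-filtered starts, with a late-match buff; respawns credit opposing teams' scores.
; Post-match, it removes all but the top scorer and notifies the UI; FlipFlop team assignment supports only two players.
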(event `self.ReceiveBeginPlay`
  ;[1 1 1] Spawning in player
  (bind _outactors (`GameplayStatics.GetAllActorsOfClass` "/Script/Engine.PlayerController"))
  (bind _output_get (set `self.NumOfPlayersToSpawn` (- (`self.NumberOfPlayers`) (`KismetArrayLibrary.Array_Length` _outactors))))
  (`/Engine/EditorBlueprintResources/StandardMacros.CompareInt` _output_get
    (:`>`
      (for _ (range 1 (+ (`self.NumOfPlayersToSpawn`) 1))
        (`GameplayStatics.CreatePlayer` -1)))
    (:`==`
      _))
  (bind _outactors_2 (`GameplayStatics.GetAllActorsOfClass` "/Script/Engine.PlayerController"))
  ;[1 1 1] Setting up UI for each player screen
  (for _array_element _outactors_2
    (bind _returnvalue (`|CreateWidget` "/Game/Student/Blueprints/Widgets/DeathMatchUI.DeathMatchUI_C" _array_element))
    (`UserWidget.AddToPlayerScreen` _returnvalue 0)
    (`WidgetBlueprintLibrary.SetInputMode_UIOnlyEx` _array_element _returnvalue)
    (if (== (`GameplayStatics.GetPlayerControllerID` _array_element) 0)
      (`KismetSystemLibrary.Delay` 0.1)
      (`Widget.SetKeyboardFocus` (`/Game/Student/Blueprints/Widgets/DeathMatchUI.Play` _returnvalue)))))

(event `self.HandleStartingNewPlayer`
  (params (NewPlayer :type "PlayerController Object Reference"))
  ;[1 1 1] Handle Starting new player
  (`/Engine/EditorBlueprintResources/StandardMacros.FlipFlop` ; Only works for 2 player games
    (:`A`
      (`self.RestartPlayer` NewPlayer))
    (:`B`
      (message `/Game/Student/Blueprints/Interfaces/I_PlayerController.SetTeam` NewPlayer "NewEnumerator1")
      (`self.RestartPlayer` NewPlayer))))

(event `RequestRespawn`
  (params (Controller :type "Controller Object Reference"))
  ;[1 1 1] Request to Respawn player
  (`KismetSystemLibrary.Delay` 1.0)
  (`self.RestartPlayer` Controller)
  (if (== (`self.GetMatchState`) "InProgress")
    (bind _team (message `/Game/Student/Blueprints/Interfaces/I_PlayerController.GetTeam` Controller))
    (bind _outactors (`GameplayStatics.GetAllActorsOfClass` "/Game/Student/Blueprints/Controllers/DMPlayerController.DMPlayerController_C"))
    (for _array_element _outactors
      (if (`|EnumInequality` (`/Game/Student/Blueprints/Controllers/DMPlayerController.Team` _array_element) _team)
        (`/Engine/EditorBlueprintResources/StandardMacros.IncrementInt` (`/Game/Student/Blueprints/Controllers/DMPlayerController.Score` _array_element))))))

(event `self.K2_OnRestartPlayer`
  (params (NewPlayer :type "Controller Object Reference"))
  ;[1 1 1] On Player Restart
  (if (== (`self.GetMatchState`) "InProgress")
    (bind _spawnedtank (message `/Game/Student/Blueprints/Interfaces/I_PlayerController.SpawnAndPossess` NewPlayer (`/Game/Student/Blueprints/MacroLibraries/GameFunctionMacros.GetRandomTankClass`) null))
    (`/Engine/EditorBlueprintResources/StandardMacros.IsValid` _spawnedtank
      (:`Is Valid`
        (`/Game/Student/Blueprints/MacroLibraries/GameFunctionMacros.EquipAllWeapons` _spawnedtank)
        (if (< (`self.MatchTimeRemaining`) 30)
          (message `/Game/Student/Blueprints/Interfaces/I_PlayerController.LastLifeBuff` NewPlayer)))
      (:`Is Not Valid`
        ;[1 1 1] Match in prrogress
        (`KismetSystemLibrary.PrintString` "BAD" true true (struct :`G` 0.66 :`B` 1.0 :`A` 1.0) 100.0)))))

(event `self.K2_OnSetMatchState`
  (params (NewState :type Name))
  (bind _matchtimeremaining (`self.MatchTimeRemaining`))
  ;[1 1 1] On Set Match State
  (`KismetSystemLibrary.PrintString` (`KismetStringLibrary.Conv_NameToString` NewState))
  (switch `name` NewState
    (:`InProgress`
      ;[1 1 1] Match in prrogress
      (`KismetSystemLibrary.RetriggerableDelay` 1.0 :!label _label)
      (if (> _matchtimeremaining 0)
        (`/Engine/EditorBlueprintResources/StandardMacros.DecrementInt` _matchtimeremaining
          (:`  `
            (goto _label)))))
    (:`WaitingPostMatch`
      ;[1 1 1] Waiting Post Match
      ;;[1 1 1] Determine the winner of the game
      (for (_array_element _array_index) (`self.PlayerControllers`)
        (if (== _array_index 0)
          (set `self.BestPlayerController` _array_element) ; Set first index to the best PC
          (else
            (`|ExecutionSequence`
              (:`then_0`
                (bind _score (message `/Game/Student/Blueprints/Interfaces/I_PlayerController.GetScore` _array_element)) ; score of current PC
                (bind _score_2 (message `/Game/Student/Blueprints/Interfaces/I_PlayerController.GetScore` (`self.BestPlayerController`))) ; score of best PC
              )
              (:`then_1`
                (if (> _score _score_2)
                  (bind _asplayer_controller (cast `PlayerController` (`self.BestPlayerController`))
                    (:`then`
                      (`GameplayStatics.RemovePlayer` _asplayer_controller true) ; remove the previous best player
                    )
                    (:`CastFailed`
                      _))
                  (set `self.BestPlayerController` _array_element) ; set current PC to best PC if higher score
                  (else
                    (bind _asplayer_controller_2 (cast `PlayerController` _array_element))
                    (`GameplayStatics.RemovePlayer` _asplayer_controller_2 true) ; Remove the current player
                  )))))))
      ;;;[1 1 1] Tell UI the winner
      (bind _foundwidgets (`WidgetBlueprintLibrary.GetAllWidgetsOfClass` "/Game/Student/Blueprints/Widgets/DeathMatchUI.DeathMatchUI_C"))
      (for _array_element_2 _foundwidgets
        (`/Game/Student/Blueprints/Interfaces/I_HUD.WinnerDetermined` _array_element_2 (`self.BestPlayerController`))))))

(event `self.K2_PostLogin`
  (params (NewPlayer :type "PlayerController Object Reference"))
  ;[1 1 1] On Player Login
  (`KismetArrayLibrary.Array_AddUnique` (`self.PlayerControllers`) NewPlayer) ; Add PC to array of PCs
)

(event `self.K2_OnLogout`
  (params (ExitingController :type "Controller Object Reference"))
  ;[1 1 1] On Player Logout
  (`KismetArrayLibrary.Array_RemoveItem` (`self.PlayerControllers`) ExitingController) ; Remove PC from array of PCs
)

(fn `BuildTeamsStartsArray`
  (params (Start :type "/Game/Student/Blueprints/Tanks/TankPlayerStart Object Reference"))
  (switch `/Game/Student/Blueprints/Tanks/TeamsList` (`/Game/Student/Blueprints/Tanks/TankPlayerStart.Team` Start)
    (:`NewEnumerator0`
      (`KismetArrayLibrary.Array_AddUnique` (`self.NoTeamPlayerStarts`) Start))
    (:`NewEnumerator1`
      (`KismetArrayLibrary.Array_AddUnique` (`self.RedPlayerStarts`) Start))
    (:`NewEnumerator2`
      (`KismetArrayLibrary.Array_AddUnique` (`self.BluePlayerStarts`) Start))))

(fn `FindPlayerStart`
  (params (Player :type "Controller Object Reference") (IncomingName :type String))
  (returns (ReturnValue :type "Actor Object Reference"))
  (bind _outactors (`GameplayStatics.GetAllActorsOfClass` "/Game/Student/Blueprints/Tanks/TankPlayerStart.TankPlayerStart_C"))
  (for _array_element _outactors
    (`self.BuildTeamsStartsArray` _array_element))
  (bind _team (message `/Game/Student/Blueprints/Interfaces/I_PlayerController.GetTeam` Player))
  (switch `/Game/Student/Blueprints/Tanks/TeamsList` _team
    (:`NewEnumerator0`
      (bind _start (`self.GetRandomStart` (`self.NoTeamPlayerStarts`)))
      (return _start))
    (:`NewEnumerator1`
      (bind _start_2 (`self.GetRandomStart` (`self.RedPlayerStarts`)))
      (return _start_2))
    (:`NewEnumerator2`
      (bind _start_3 (`self.GetRandomStart` (`self.BluePlayerStarts`)))
      (return _start_3))))

(fn `GetRandomStart`
  (params (Starts :type "Array of /Game/Student/Blueprints/Tanks/TankPlayerStart Object Reference"))
  (returns (Start :type "/Game/Student/Blueprints/Tanks/TankPlayerStart Object Reference"))
  (return (`|GetArrayItem` Starts (`KismetMathLibrary.RandomIntegerInRange` 0 (`KismetArrayLibrary.Array_LastIndex` Starts)))))

(fn `GetTimeRemaining`
  (returns (TimeRemaining :type Integer))
  (return (`self.MatchTimeRemaining`)))

(fn `ReadyToEndMatch`
  (returns (ReturnValue :type Boolean))
  (return (<= (`self.MatchTimeRemaining`) 0)))

(fn `ReadyToStartMatch`
  (returns (ReturnValue :type Boolean))
  ;[1 1 1] If anyone isnt ready, return false
  (for _array_element (`self.PlayerControllers`)
    (bind _ready (message `/Game/Student/Blueprints/Interfaces/I_PlayerController.IsReady` _array_element))
    (if (not _ready)
      (return false)))
  (bind _foundwidgets (`WidgetBlueprintLibrary.GetAllWidgetsOfClass` "/Game/Student/Blueprints/Widgets/DeathMatchUI.DeathMatchUI_C"))
  (for _array_element_2 _foundwidgets
    (`/Game/Student/Blueprints/Widgets/DeathMatchUI.PlayersReady` _array_element_2))
  (return true))

(fn `UserConstructionScript`)