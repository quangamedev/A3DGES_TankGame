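; CollectingGameMode is a game mode for a gem-collecting match that declares a winner once a player reaches a gem target.
; On BeginPlay it finds every GemPickUp in the level and binds to its gem-collected event.
; Each pickup passes its gem value to the collector's CollectingPlayerControlller, whose returned count is compared with GemsToWin.
; Reaching the target calls Win, which only prints the winning controller's name.
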(event `self.ReceiveBeginPlay`
  (bind _outactors (`GameplayStatics.GetAllActorsOfClass` "/Game/Student/Blueprints/PickUps/GemPickUp.GemPickUp_C"))
  (for _array_element _outactors
    (add `/Game/Student/Blueprints/PickUps/GemPickUp.OnGemCollected` _array_element (`|CreateDelegate` :!event `GemPickedUp`))))

(event `GemPickedUp`
  (params (Causer :type "Actor Object Reference") (GemRef :type "/Game/Student/Blueprints/PickUps/GemPickUp Object Reference"))
  (bind _returnvalue (`self.GetInstigatorController` Causer))
  (bind _ascollecting_player_controlller (cast `/Game/Student/Blueprints/Controllers/CollectingPlayerControlller` _returnvalue))
  (bind _numberofgems (`/Game/Student/Blueprints/Controllers/CollectingPlayerControlller.GemCollected` _ascollecting_player_controlller (`/Game/Student/Blueprints/PickUps/GemPickUp.GemsToAdd` GemRef)))
  (if (>= _numberofgems (`self.GemsToWin`))
    (`self.Win` _returnvalue)))

(event `Win`
  (params (Winner :type "Actor Object Reference"))
  (`KismetSystemLibrary.PrintString` (`KismetStringLibrary.Concat_StrStr` "Winner is: " (`KismetSystemLibrary.GetDisplayName` Winner))))

(fn `UserConstructionScript`)