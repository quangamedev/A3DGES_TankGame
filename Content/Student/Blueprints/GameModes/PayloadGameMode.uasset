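; Game mode for a local multiplayer Payload tank match, won when the cart completes its track and lost if it is destroyed.
; BeginPlay binds cart events, creates local players from the "players" option and gives each a PayloadUI; the match starts once all are ready.
; Players join Blue, spawn at random team starts with random weapons and get a last-life buff when cart health is low.
; At match end, each UI receives the result and top-scoring MVP.
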(event `self.ReceiveBeginPlay`
  (bind _returnvalue (`KismetStringLibrary.Conv_StringToInt` (`GameplayStatics.ParseOption` (`self.OptionsString`) "players")))
  (bind _outactors (`GameplayStatics.GetAllActorsOfClass` "/Game/Student/Blueprints/Payload/PayloadCart.PayloadCart_C"))
  (bind _output_get (set `self.PayloadRef` (`|GetArrayItem` _outactors)))
  ;[1 1 1] Spawning in player
  (add `/Game/Student/Blueprints/Payload/PayloadCart.OnCartDestroyed` _output_get (`|CreateDelegate` :!event `LoseGame`))
  (add `/Game/Student/Blueprints/Payload/PayloadCart.OnTrackCompleted` _output_get (`|CreateDelegate` :!event `WinGame`))
  (if (not (== _returnvalue 0))
    (set `self.NumberOfPlayers` _returnvalue))
  (bind _outactors_2 (`GameplayStatics.GetAllActorsOfClass` "/Script/Engine.PlayerController"))
  (bind _output_get_2 (set `self.NumOfPlayersToSpawn` (- (`self.NumberOfPlayers`) (`KismetArrayLibrary.Array_Length` _outactors_2))))
  (`/Engine/EditorBlueprintResources/StandardMacros.CompareInt` _output_get_2
    (:`>`
      (for _ (range 1 (+ (`self.NumOfPlayersToSpawn`) 1))
        (`GameplayStatics.CreatePlayer` -1)))
    (:`==`
      _))
  (bind _outactors_3 (`GameplayStatics.GetAllActorsOfClass` "/Script/Engine.PlayerController"))
  ;[1 1 1] Setting up UI for each player screen
  (for _array_element _outactors_3
    (bind _returnvalue_2 (`|CreateWidget` "/Game/Student/Blueprints/Widgets/PayloadUI.PayloadUI_C" _array_element))
    (`UserWidget.AddToPlayerScreen` _returnvalue_2 0)
    (`WidgetBlueprintLibrary.SetInputMode_UIOnlyEx` _array_element _returnvalue_2)
    (if (== (`GameplayStatics.GetPlayerControllerID` _array_element) 0)
      (`KismetSystemLibrary.Delay` 0.1)
      (`Widget.SetKeyboardFocus` (`/Game/Student/Blueprints/Widgets/PayloadUI.Play` _returnvalue_2)))))

(event `WinGame`
  (set `self.CartReachedDestination` true))

(event `LoseGame`
  (set `self.CartDestroyed` true))

(event `self.HandleStartingNewPlayer`
  (params (NewPlayer :type "PlayerController Object Reference"))
  ;[1 1 1] Handle Starting new player
  (message `/Game/Student/Blueprints/Interfaces/I_PlayerController.SetTeam` NewPlayer "NewEnumerator2")
  (`self.RestartPlayer` NewPlayer))

(event `RequestRespawn`
  (params (Controller :type "Controller Object Reference"))
  ;[1 1 1] Request to Respawn player
  (`KismetSystemLibrary.Delay` 1.0)
  (`self.RestartPlayer` Controller))

(event `AddScoreTo`
  (params (Controller :type "Controller Object Reference"))
  ;[1 1 1] Add score to controller
  (if (== (`self.GetMatchState`) "InProgress")
    (bind _aspayload_player_controller (cast `/Game/Student/Blueprints/Controllers/PayloadPlayerController` Controller))
    (`/Engine/EditorBlueprintResources/StandardMacros.IncrementInt` (`/Game/Student/Blueprints/Controllers/PayloadPlayerController.Score` _aspayload_player_controller))))

(event `self.K2_OnRestartPlayer`
  (params (NewPlayer :type "Controller Object Reference"))
  (bind _payloadref (`self.PayloadRef`))
  ;[1 1 1] On Player Restart
  (if (== (`self.GetMatchState`) "InProgress")
    (bind _currenttank (message `/Game/Student/Blueprints/Interfaces/I_PlayerController.GetCurrentTank` NewPlayer))
    (bind _spawnedtank (message `/Game/Student/Blueprints/Interfaces/I_PlayerController.SpawnAndPossess` NewPlayer _currenttank null))
    (`/Engine/EditorBlueprintResources/StandardMacros.IsValid` _spawnedtank
      (:`Is Valid`
        (`/Game/Student/Blueprints/MacroLibraries/GameFunctionLibrary.EquipRandomWeapon` _spawnedtank false)
        (if (< (`KismetMathLibrary.MapRangeClamped` (`/Game/Student/Blueprints/Payload/PayloadCart.Health` _payloadref) 0.0 (`/Game/Student/Blueprints/Payload/PayloadCart.MaxHealth` _payloadref) 0.0 1.0) 0.15)
          (message `/Game/Student/Blueprints/Interfaces/I_PlayerController.LastLifeBuff` NewPlayer)))
      (:`Is Not Valid`
        (message `/Game/Student/Blueprints/Interfaces/I_PlayerController.EnableRespawnButton` NewPlayer)))))

(event `self.K2_OnSetMatchState`
  (params (NewState :type Name))
  ;[1 1 1] On Set Match State
  (`KismetSystemLibrary.PrintString` (`KismetStringLibrary.Conv_NameToString` NewState))
  (switch `name` NewState
    (:`WaitingPostMatch`
      ;[1 1 1] Waiting Post Match
      (for (_array_element _array_index) (`self.PlayerControllers`)
        (if (== _array_index 0)
          (set `self.BestPlayerController` _array_element) ; Set first index to the best PC
          (else
            (`|ExecutionSequence`
              (:`then_0`
                (bind _score (message `/Game/Student/Blueprints/Interfaces/I_PlayerController.GetScore` _array_element)) ; score of current PC
                (bind _score_2 (message `/Game/Student/Blueprints/Interfaces/I_PlayerController.GetScore` (`self.BestPlayerController`))) ; score of best PC
              )
              (:`then_1`
                (if (> _score _score_2)
                  (set `self.BestPlayerController` _array_element) ; set current PC to best PC if higher score
                ))))))
      ;;[1 1 1] Tell UI the result
      (bind _foundwidgets (`WidgetBlueprintLibrary.GetAllWidgetsOfClass` "/Game/Student/Blueprints/Widgets/PayloadUI.PayloadUI_C"))
      (for _array_element_2 _foundwidgets
        (message `/Game/Student/Blueprints/Interfaces/I_HUD.PayloadGameEnded` _array_element_2 (`self.CartReachedDestination`) (`self.BestPlayerController`))))))

(event `self.K2_PostLogin`
  (params (NewPlayer :type "PlayerController Object Reference"))
  ;[1 1 1] On Player Login
  (`KismetArrayLibrary.Array_AddUnique` (`self.PlayerControllers`) NewPlayer) ; Add PC to array of PCs
)

(event `self.K2_OnLogout`
  (params (ExitingController :type "Controller Object Reference"))
  ;[1 1 1] On Player Logout
  (`KismetArrayLibrary.Array_RemoveItem` (`self.PlayerControllers`) ExitingController) ; Remove PC from array of PCs
)

(fn `BuildTeamsStartsArray`
  (params (Start :type "/Game/Student/Blueprints/Tanks/TankPlayerStart Object Reference"))
  (switch `/Game/Student/Blueprints/Tanks/TeamsList` (`/Game/Student/Blueprints/Tanks/TankPlayerStart.Team` Start)
    (:`NewEnumerator0`
      (`KismetArrayLibrary.Array_AddUnique` (`self.NoTeamPlayerStarts`) Start))
    (:`NewEnumerator1`
      (`KismetArrayLibrary.Array_AddUnique` (`self.RedPlayerStarts`) Start))
    (:`NewEnumerator2`
      (`KismetArrayLibrary.Array_AddUnique` (`self.BluePlayerStarts`) Start))))

(fn `FindPlayerStart`
  (params (Player :type "Controller Object Reference") (IncomingName :type String))
  (returns (ReturnValue :type "Actor Object Reference"))
  (bind _outactors (`GameplayStatics.GetAllActorsOfClass` "/Game/Student/Blueprints/Tanks/TankPlayerStart.TankPlayerStart_C"))
  (for _array_element _outactors
    (`self.BuildTeamsStartsArray` _array_element))
  (bind _team (message `/Game/Student/Blueprints/Interfaces/I_PlayerController.GetTeam` Player))
  (switch `/Game/Student/Blueprints/Tanks/TeamsList` _team
    (:`NewEnumerator0`
      (bind _start (`self.GetRandomStart` (`self.NoTeamPlayerStarts`)))
      (return _start))
    (:`NewEnumerator1`
      (bind _start_2 (`self.GetRandomStart` (`self.RedPlayerStarts`)))
      (return _start_2))
    (:`NewEnumerator2`
      (bind _start_3 (`self.GetRandomStart` (`self.BluePlayerStarts`)))
      (return _start_3))))

(fn `GetPayloadCartRef`
  (returns (PayloadCartRef :type "/Game/Student/Blueprints/Payload/PayloadCart Object Reference"))
  (return (`self.PayloadRef`)))

(fn `GetRandomStart`
  (params (Starts :type "Array of /Game/Student/Blueprints/Tanks/TankPlayerStart Object Reference"))
  (returns (Start :type "/Game/Student/Blueprints/Tanks/TankPlayerStart Object Reference"))
  (return (`|GetArrayItem` Starts (`KismetMathLibrary.RandomIntegerInRange` 0 (`KismetArrayLibrary.Array_LastIndex` Starts)))))

(fn `GetTimeRemaining`
  (returns (TimeRemaining :type Integer))
  (return 0))

(fn `ReadyToEndMatch`
  (returns (ReturnValue :type Boolean))
  (return (or (`self.CartReachedDestination`) (`self.CartDestroyed`))))

(fn `ReadyToStartMatch`
  (returns (ReturnValue :type Boolean))
  ;[1 1 1] If anyone isnt ready, return false
  (for _array_element (`self.PlayerControllers`)
    (bind _ready (message `/Game/Student/Blueprints/Interfaces/I_PlayerController.IsReady` _array_element))
    (if (not _ready)
      (return false)))
  (bind _foundwidgets (`WidgetBlueprintLibrary.GetAllWidgetsOfClass` "/Game/Student/Blueprints/Widgets/PayloadUI.PayloadUI_C"))
  (for _array_element_2 _foundwidgets
    (`/Game/Student/Blueprints/Widgets/DeathMatchUI.PlayersReady` _array_element_2))
  (return true))

(fn `UserConstructionScript`)