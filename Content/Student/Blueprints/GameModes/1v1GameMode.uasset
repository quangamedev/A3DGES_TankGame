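; Game mode for local multiplayer 1v1 tank matches with team starts, limited lives and a last-player-standing winner.
; BeginPlay creates missing players and their UI widgets, and the match starts once all controllers report ready.
; A two-player-only FlipFlop puts the second player on Red, and spawns pick random team-matching TankPlayerStarts.
; Respawns spawn the player's current tank, buffing the last life; out-of-lives players are removed until one remains.
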(event `self.ReceiveBeginPlay`
  (bind _outactors (`GameplayStatics.GetAllActorsOfClass` "/Script/Engine.PlayerController"))
  (bind _output_get (set `self.NumOfPlayersToSpawn` (- (`self.NumberOfPlayers`) (`KismetArrayLibrary.Array_Length` _outactors))))
  (`/Engine/EditorBlueprintResources/StandardMacros.CompareInt` _output_get
    (:`>`
      (for _ (range 1 (+ (`self.NumOfPlayersToSpawn`) 1))
        (`GameplayStatics.CreatePlayer` -1)))
    (:`==`
      _))
  (bind _outactors_2 (`GameplayStatics.GetAllActorsOfClass` "/Script/Engine.PlayerController"))
  (for _array_element _outactors_2
    (bind _returnvalue (`|CreateWidget` "/Game/Student/Blueprints/Widgets/GameModeUI.GameModeUI_C" _array_element))
    (`UserWidget.AddToPlayerScreen` _returnvalue 0)
    (`WidgetBlueprintLibrary.SetInputMode_UIOnlyEx` _array_element _returnvalue)
    (if (== (`GameplayStatics.GetPlayerControllerID` _array_element) 0)
      (`KismetSystemLibrary.Delay` 0.1)
      (`Widget.SetKeyboardFocus` (`/Game/Student/Blueprints/Widgets/GameModeUI.Play` _returnvalue)))))

(event `self.HandleStartingNewPlayer`
  (params (NewPlayer :type "PlayerController Object Reference"))
  (`/Engine/EditorBlueprintResources/StandardMacros.FlipFlop` ; Only works for 2 player games
    (:`A`
      (`self.RestartPlayer` NewPlayer))
    (:`B`
      (message `/Game/Student/Blueprints/Interfaces/I_PlayerController.SetTeam` NewPlayer "NewEnumerator1")
      (`self.RestartPlayer` NewPlayer))))

(event `RequestRespawn`
  (params (Controller :type "Controller Object Reference"))
  (bind _lives (message `/Game/Student/Blueprints/Interfaces/I_PlayerController.GetLives` Controller))
  (if (> _lives 0)
    (`KismetSystemLibrary.Delay` 1.0)
    (`self.RestartPlayer` Controller)
    (else
      (bind _asplayer_controller (cast `PlayerController` Controller))
      (`GameplayStatics.RemovePlayer` _asplayer_controller))))

(event `self.K2_OnRestartPlayer`
  (params (NewPlayer :type "Controller Object Reference"))
  (bind _lives (message `/Game/Student/Blueprints/Interfaces/I_PlayerController.GetLives` NewPlayer))
  (bind _currenttank (message `/Game/Student/Blueprints/Interfaces/I_PlayerController.GetCurrentTank` NewPlayer))
  (message `/Game/Student/Blueprints/Interfaces/I_PlayerController.SpawnAndPossess` NewPlayer _currenttank null)
  (if (== _lives 1)
    (message `/Game/Student/Blueprints/Interfaces/I_PlayerController.LastLifeBuff` NewPlayer)))

(event `self.K2_OnSetMatchState`
  (params (NewState :type Name))
  (`KismetSystemLibrary.PrintString` (`KismetStringLibrary.Conv_NameToString` NewState))
  (switch `name` NewState))

(event `self.K2_PostLogin`
  (params (NewPlayer :type "PlayerController Object Reference"))
  (`KismetArrayLibrary.Array_AddUnique` (`self.PlayerControllers`) NewPlayer))

(event `self.K2_OnLogout`
  (params (ExitingController :type "Controller Object Reference"))
  (`KismetArrayLibrary.Array_RemoveItem` (`self.PlayerControllers`) ExitingController)
  (if (== (`KismetArrayLibrary.Array_Length` (`self.PlayerControllers`)) 1)
    (`KismetSystemLibrary.PrintString` (`KismetStringLibrary.Concat_StrStr` "The winner is: " (`KismetSystemLibrary.GetDisplayName` (`|GetArrayItem` (`self.PlayerControllers`)))) false)
    (bind _foundwidgets (`WidgetBlueprintLibrary.GetAllWidgetsOfClass` "/Game/Student/Blueprints/Widgets/GameModeUI.GameModeUI_C"))
    (for _array_element _foundwidgets
      (`/Game/Student/Blueprints/Interfaces/I_HUD.WinnerDetermined` _array_element (`|GetArrayItem` (`self.PlayerControllers`))))))

(fn `BuildTeamsStartsArray`
  (params (Start :type "/Game/Student/Blueprints/Tanks/TankPlayerStart Object Reference"))
  (switch `/Game/Student/Blueprints/Tanks/TeamsList` (`/Game/Student/Blueprints/Tanks/TankPlayerStart.Team` Start)
    (:`NewEnumerator0`
      (`KismetArrayLibrary.Array_AddUnique` (`self.NoTeamPlayerStarts`) Start))
    (:`NewEnumerator1`
      (`KismetArrayLibrary.Array_AddUnique` (`self.RedPlayerStarts`) Start))
    (:`NewEnumerator2`
      (`KismetArrayLibrary.Array_AddUnique` (`self.BluePlayerStarts`) Start))))

(fn `FindPlayerStart`
  (params (Player :type "Controller Object Reference") (IncomingName :type String))
  (returns (ReturnValue :type "Actor Object Reference"))
  (bind _outactors (`GameplayStatics.GetAllActorsOfClass` "/Game/Student/Blueprints/Tanks/TankPlayerStart.TankPlayerStart_C"))
  (for _array_element _outactors
    (`self.BuildTeamsStartsArray` _array_element))
  (bind _team (message `/Game/Student/Blueprints/Interfaces/I_PlayerController.GetTeam` Player))
  (switch `/Game/Student/Blueprints/Tanks/TeamsList` _team
    (:`NewEnumerator0`
      (bind _start (`self.GetRandomStart` (`self.NoTeamPlayerStarts`)))
      (return _start))
    (:`NewEnumerator1`
      (bind _start_2 (`self.GetRandomStart` (`self.RedPlayerStarts`)))
      (return _start_2))
    (:`NewEnumerator2`
      (bind _start_3 (`self.GetRandomStart` (`self.BluePlayerStarts`)))
      (return _start_3))))

(fn `GetRandomStart`
  (params (Starts :type "Array of /Game/Student/Blueprints/Tanks/TankPlayerStart Object Reference"))
  (returns (Start :type "/Game/Student/Blueprints/Tanks/TankPlayerStart Object Reference"))
  (return (`|GetArrayItem` Starts (`KismetMathLibrary.RandomIntegerInRange` 0 (`KismetArrayLibrary.Array_LastIndex` Starts)))))

(fn `ReadyToEndMatch`
  (returns (ReturnValue :type Boolean))
  (return (== (`KismetArrayLibrary.Array_Length` (`self.PlayerControllers`)) 1)))

(fn `ReadyToStartMatch`
  (returns (ReturnValue :type Boolean))
  ;[1 1 1] If anyone isnt ready, return false
  (for _array_element (`self.PlayerControllers`)
    (bind _ready (message `/Game/Student/Blueprints/Interfaces/I_PlayerController.IsReady` _array_element))
    (if (not _ready)
      (return false)))
  (bind _foundwidgets (`WidgetBlueprintLibrary.GetAllWidgetsOfClass` "/Game/Student/Blueprints/Widgets/GameModeUI.GameModeUI_C"))
  (for _array_element_2 _foundwidgets
    (`/Game/Student/Blueprints/Widgets/GameModeUI.PlayersReady` _array_element_2))
  (return true))

(fn `UserConstructionScript`)