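; SpawningGameMode is a game mode that spawns each player at a random start point belonging to their team.
; New players are restarted on join, and the FindPlayerStart override gathers all TankPlayerStart actors into No Team, Red and Blue arrays.
; It then reads the controller's team through a GetTeamMessage call and returns a random entry from the matching array.
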(event `self.HandleStartingNewPlayer`
  (params (NewPlayer :type "PlayerController Object Reference"))
  (`self.RestartPlayer` NewPlayer))

(fn `BuildTeamsStartsArray`
  (params (Start :type "/Game/Student/Blueprints/Tanks/TankPlayerStart Object Reference"))
  (switch `/Game/Student/Blueprints/Tanks/TeamsList` (`/Game/Student/Blueprints/Tanks/TankPlayerStart.Team` Start)
    (:`NewEnumerator0`
      (`KismetArrayLibrary.Array_AddUnique` (`self.NoTeamPlayerStarts`) Start))
    (:`NewEnumerator1`
      (`KismetArrayLibrary.Array_AddUnique` (`self.RedPlayerStarts`) Start))
    (:`NewEnumerator2`
      (`KismetArrayLibrary.Array_AddUnique` (`self.BluePlayerStarts`) Start))))

(fn `FindPlayerStart`
  (params (Player :type "Controller Object Reference") (IncomingName :type String))
  (returns (ReturnValue :type "Actor Object Reference"))
  (bind _outactors (`GameplayStatics.GetAllActorsOfClass` "/Game/Student/Blueprints/Tanks/TankPlayerStart.TankPlayerStart_C"))
  (for _array_element _outactors
    (`self.BuildTeamsStartsArray` _array_element))
  (bind _team (message `/Game/Student/Blueprints/Interfaces/I_TeamPlayerController.GetTeam` Player))
  (switch `/Game/Student/Blueprints/Tanks/TeamsList` _team
    (:`NewEnumerator0`
      (bind _start (`self.GetRandomStart` (`self.NoTeamPlayerStarts`)))
      (return _start))
    (:`NewEnumerator1`
      (bind _start_2 (`self.GetRandomStart` (`self.RedPlayerStarts`)))
      (return _start_2))
    (:`NewEnumerator2`
      (bind _start_3 (`self.GetRandomStart` (`self.BluePlayerStarts`)))
      (return _start_3))))

(fn `GetRandomStart`
  (params (Starts :type "Array of /Game/Student/Blueprints/Tanks/TankPlayerStart Object Reference"))
  (returns (Start :type "/Game/Student/Blueprints/Tanks/TankPlayerStart Object Reference"))
  (return (`|GetArrayItem` Starts (`KismetMathLibrary.RandomIntegerInRange` 0 (`KismetArrayLibrary.Array_LastIndex` Starts)))))

(fn `UserConstructionScript`)